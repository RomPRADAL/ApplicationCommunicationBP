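; BP_Interrupteur is a switch that triggers linked actors when the third-person character overlaps its box.
; If the switch is toggled on, Activate sends ToggleMessage to each Activables entry implementing BPI_Activable; otherwise it only prints that it is off.
; A separate Toggle event flips the switch's on/off state, while Desactivate is an empty stub.
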(event OnComponentBeginOverlap(Box)
  (params (OverlappedComponent :type Primitive%20Component%20Object%20Reference) (OtherActor :type Actor%20Object%20Reference) (OtherComp :type Primitive%20Component%20Object%20Reference) (OtherBodyIndex :type Integer) (bFromSweep :type Boolean) (SweepResult :type Hit%20Result%20Structure%20%28by%20ref%29))
  (Utilities|Casting|CastToBP_ThirdPersonCharacter OtherActor)
  (CallFunction|Activate))

(event EventBeginPlay)

(event Collision|EventActorBeginOverlap
  (params (OtherActor :type Actor%20Object%20Reference)))

(event EventTick
  (params (DeltaSeconds :type Float%20%28single-precision%29)))

(event EventActivate
  (if (Variables|Default|GetToggledOn)
    (for _array_element (Variables|Default|GetActivables)
      (if (Utilities|DoesObjectImplementInterface _array_element "/Game/Elements/BPI_Activable.BPI_Activable_C")
        (Class|BPIActivable|Toggle(Message) _array_element)))
    (else
      (Development|PrintString "Interrupteur éteint"))))

(event EventDesactivate)

(event EventToggle
  ;[1 1 1] Interurpteur Allumé/Eteint
  (Variables|Default|SetToggledOn (not (Variables|Default|GetToggledOn))))

(fn ConstructionScript)