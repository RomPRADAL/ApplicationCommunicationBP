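; BP_Lampe is a lamp whose point light turns on when its count of closed doors drops to zero or below.
; On BeginPlay it binds to the opening and closing events of every entry in EventLaunchers.
; Each event prints a debug message, decrements or increments NombrePortesFermee, then calls CheckLightState to update the light's visibility.
; The light state is only evaluated on door events, not at startup.
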(event Custom|UnePorteSeFerme
  (bind _nombreportesfermee (Variables|Default|GetNombrePortesFermee))
  (Development|PrintString (Utilities|String|Append "Porte se ferme  : " (Utilities|String|ToString(Integer) _nombreportesfermee)))
  (Math|Integer|IncrementInt _nombreportesfermee
    (:%20%20
      (CallFunction|CheckLightState))))

(event Custom|UnePorteS'ouvre
  (bind _nombreportesfermee (Variables|Default|GetNombrePortesFermee))
  (Development|PrintString (Utilities|String|Append "Porte s'ouvre : " (Utilities|String|ToString(Integer) _nombreportesfermee)))
  (Math|Integer|DecrementInt _nombreportesfermee
    (:%20%20
      (CallFunction|CheckLightState))))

(event EventBeginPlay
  (for _array_element (Variables|Default|GetEventLaunchers)
    (EventDispatchers|BindEventtoOuverture _array_element (delegate Custom|UnePorteS'ouvre))
    (EventDispatchers|BindEventtoFermeture _array_element (delegate Custom|UnePorteSeFerme))))

(fn ConstructionScript)

(fn CheckLightState
  (bind _pointlight (Variables|Default|GetPointLight))
  (if (<= (Variables|Default|GetNombrePortesFermee) 0)
    (Rendering|SetVisibility _pointlight true false)
    (else
      (Rendering|SetVisibility _pointlight false false))))